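; Manager actor that runs endless enemy waves from the BP_EnemySpawner actors in the level.
; On BeginPlay it caches all spawners, then spawns one BP_Enemy at each spawner's transform, passing itself as that enemy's Manager and counting it.
; RemoveEnemyAndCheck decrements the live count and, when none remain, waits briefly before spawning the next wave.
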(event Custom|Spawn%20Enemies
  (for _array_element (Variables|Default|GetSpawners)
    (bind _returnvalue (Game|SpawnActorfromClass "/Game/Blueprints/Enemies/BP_Enemy.BP_Enemy_C" (Math|Transform|MakeTransform (.location (Transformation|GetWorldTransform (Variables|/Game/Blueprints/Enemies/BP_EnemySpawner.BP_EnemySpawner_C|GetDefaultSceneRoot _array_element))) (.rotation (Transformation|GetWorldTransform (Variables|/Game/Blueprints/Enemies/BP_EnemySpawner.BP_EnemySpawner_C|GetDefaultSceneRoot _array_element))) "1.000000,1.000000,1.000000") "Undefined" "MultiplyWithRoot" 0 0)) ; Create new enemy at the spawners location and rotation
    (Variables|/Game/Blueprints/Enemies/BP_Enemy.BP_Enemy_C|SetManager _returnvalue self) ; Assign this manager to the manager variable an each enemy
    (Math|Integer|IncrementInt (Variables|Default|GetCurrentEnemyTotal))))

(event Custom|Remove%20EnemyAndCheck
  (Math|Integer|DecrementInt (Variables|Default|GetCurrentEnemyTotal)
    (:%20%20
      (if (not (> (Variables|Default|GetCurrentEnemyTotal) 0))
        (Development|PrintString "New Wave Incoming")
        (Utilities|FlowControl|Delay 5.0)
        (CallFunction|SpawnEnemies)))))

(event EventBeginPlay
  (Development|PrintString "Enemy Spawn Manager is ready")
  (bind _outactors (Actor|GetAllActorsOfClass "/Game/Blueprints/Enemies/BP_EnemySpawner.BP_EnemySpawner_C"))
  (Variables|Default|SetSpawners _outactors)
  (CallFunction|SpawnEnemies))

(event Collision|EventActorBeginOverlap
  (params (OtherActor :type Actor%20Object%20Reference)))

(event EventTick
  (params (DeltaSeconds :type Float%20%28single-precision%29)))

(fn ConstructionScript)